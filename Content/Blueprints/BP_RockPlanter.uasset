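; BP_RockPlanter is a pickup item that the third-person character carries to plant rocks in the world.
; On overlap it stores the character and passes itself to PickUpItem, and its PickUp event attaches it to the left-hand socket.
; PlantSeed traces downward and spawns an actor, with no class set in the graph, at the hit location with random yaw and height scale.
; Drop only prints a message.
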(event `self.ReceiveActorBeginOverlap`
  (params (OtherActor :type "Actor Object Reference"))
  (bind _asbp_third_person_character (cast `/Game/ThirdPerson/Blueprints/BP_ThirdPersonCharacter` OtherActor))
  (set `self.Player` _asbp_third_person_character)
  (`/Game/ThirdPerson/Blueprints/BP_ThirdPersonCharacter.PickUpItem` _asbp_third_person_character self))

(event `/Game/Blueprints/I_SeedPlanter.PickUp`
  (`KismetSystemLibrary.PrintText` "This rock Planter has been picked up!")
  (`self.K2_AttachToComponent` (`Character.Mesh` (`self.Player`)) "hand_l" "SnapToTarget" "SnapToTarget" "KeepRelative"))

(event `/Game/Blueprints/I_SeedPlanter.PlantSeed`
  (bind _returnvalue (`self.K2_GetActorLocation`))
  (`KismetSystemLibrary.PrintText` "Trying to plant rocks!")
  (bind _outhit (`KismetSystemLibrary.LineTraceSingle` _returnvalue (+ _returnvalue (0.0 0.0 -200.0)) "TraceTypeQuery1" false (`|MakeArray` (`self.Player`)) "ForDuration"))
  (`|SpawnActorFromClass` "/Game/Blueprints/BP_Tree.BP_Tree_C" (`KismetMathLibrary.MakeTransform` (`.Location` (`GameplayStatics.BreakHitResult` _outhit)) (`KismetMathLibrary.MakeRotator` 0.0 0.0 (`KismetMathLibrary.RandomFloatInRange` 0.0 360.0)) (`KismetMathLibrary.MakeVector` 1.0 1.0 (`KismetMathLibrary.RandomFloatInRange` 0.7 1.2))) "Undefined" "MultiplyWithRoot" null null))

(event `/Game/Blueprints/I_SeedPlanter.Drop`
  (`KismetSystemLibrary.PrintText` "Trying to drop the planter"))

(fn `UserConstructionScript`)
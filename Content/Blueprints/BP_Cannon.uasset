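; BP_Cannon is a cannon actor that fires when overlapped, pushing a third-person character along the spawn point's forward vector.
; Overlap, and a one-second test delay on BeginPlay, call LaunchCannonball, which only prints text; the cannonball spawn node is unconnected.
; If the overlapping actor is the character, ActivationPlatform starts simulating physics and receives a mass-independent force along with the character's capsule.
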(event `self.ReceiveBeginPlay`
  (`KismetSystemLibrary.Delay` 1.0) ; Testing purposes only
  (`self.Launch Cannonball` :!label _label)
  (bind _asbp_third_person_character (cast `/Game/ThirdPerson/Blueprints/BP_ThirdPersonCharacter` (stale `self.ReceiveActorBeginOverlap` OtherActor)))
  (`PrimitiveComponent.SetSimulatePhysics` (`self.ActivationPlatform`) true)
  (`PrimitiveComponent.AddForce` (`Character.CapsuleComponent` _asbp_third_person_character) (* (`SceneComponent.GetForwardVector` (`self.BoxSpawnPoint`)) (`self.Force`)) "None" true)
  (`PrimitiveComponent.AddForce` (`self.ActivationPlatform`) (* (`SceneComponent.GetForwardVector` (`self.BoxSpawnPoint`)) (`self.Force`)) "None" true))

(event `self.ReceiveActorBeginOverlap`
  (params (OtherActor :type "Actor Object Reference"))
  (goto _label))

(event `Launch Cannonball`
  (`KismetSystemLibrary.PrintText` "Ka-pow!"))

(fn `UserConstructionScript`)
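; BP_Tree is a tree actor that grows in size over time after play begins.
; While GrowCounter is above zero, BeginPlay waits a random few seconds, adds a random increment to the static mesh's relative scale, then decrements the counter.
; The growth repeats by wiring execution back to the counter check through a latent Delay, with no Tick or timer.
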(event `self.ReceiveBeginPlay`
  (bind _staticmesh (`self.StaticMesh`))
  (if (> (`self.GrowCounter`) 0) :!label _label
    ; Comment
    (`KismetSystemLibrary.Delay` (`KismetMathLibrary.RandomFloatInRange` 4.0 6.0))
    (`SceneComponent.SetRelativeScale3D` _staticmesh (+ (`SceneComponent.RelativeScale3D` _staticmesh) (`KismetMathLibrary.RandomFloatInRange` 0.2 0.4)))
    (`/Engine/EditorBlueprintResources/StandardMacros.DecrementInt` (`self.GrowCounter`) ; subtract 1 from \ngrow counter
      (:`  `
        (goto _label)))))

(fn `UserConstructionScript`)
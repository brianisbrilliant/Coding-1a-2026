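; BP_Door is a door actor that swings open when the player character overlaps it, spending one of the character's keys if it is locked.
; A timeline lerps the mesh yaw to open it, with a slightly pitch-randomized sound.
; Leaving the overlap box reverses the timeline when unlocked, without checking who left.
; Locked and unlock messages are printed, and a reversed-sound closing branch is left disconnected.
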(event `self.ReceiveActorBeginOverlap`
  (params (OtherActor :type "Actor Object Reference"))
  (bind _asbp_third_person_character (cast `/Game/ThirdPerson/Blueprints/BP_ThirdPersonCharacter` OtherActor)) ; is it the player that ran into us?
  (if (`self.locked`)
    (if (> (`/Game/ThirdPerson/Blueprints/BP_ThirdPersonCharacter.TotalKeys` _asbp_third_person_character) 0)
      ; unlocking the door
      (`/Engine/EditorBlueprintResources/StandardMacros.DecrementInt` (`/Game/ThirdPerson/Blueprints/BP_ThirdPersonCharacter.TotalKeys` _asbp_third_person_character) ; subtract 1 from totalKeys
        (:`  `
          (`KismetSystemLibrary.PrintText` "unlocking door!")
          (set `self.locked` false)
          (`GameplayStatics.PlaySoundAtLocation` "/Game/Audio/Wallace_s_Mechanical_Toys_Sound_Pack/03_Bells/Bell_Crowbar.Bell_Crowbar" (`self.K2_GetActorLocation`) (struct) 1.0 (`KismetMathLibrary.RandomFloatInRange` 0.98 1.02) 0.0 "/Game/Audio/ATT_Default.ATT_Default" null null null :!label _label)
          (bind (_direction _newtrack_0) (`Timeline|swing door open` :!label _label_2)
            (:`Update`
              (`SceneComponent.K2_SetRelativeRotation` (`self.SM_Bld_Door_01`) (`KismetMathLibrary.MakeRotator` 0.0 0.0 (`KismetMathLibrary.Lerp` 0.0 -90.0 _newtrack_0)) false false)))))
      (else
        (`KismetSystemLibrary.PrintText` "I am locked!")))
    (else
      (goto _label))))

(event `self.OverlapBox.OnComponentEndOverlap`
  (params (OverlappedComponent :type "PrimitiveComponent Object Reference") (OtherActor :type "Actor Object Reference") (OtherComp :type "PrimitiveComponent Object Reference") (OtherBodyIndex :type Integer))
  (if (not (`self.locked`))
    (goto _label_2 :!via `Reverse`)))

(fn `UserConstructionScript`)